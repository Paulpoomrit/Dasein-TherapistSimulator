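; Base mixed-reality spawner that places a single object of a configurable class on room surfaces using the left controller trigger.
; Trigger events raycast from the left aim through MRUK to position a preview indicator, facing the player or following the surface normal.
; Completing the trigger spawns the object at the preview or teleports the existing one, with sound and haptics.
; The floor-only option actually tests for GLOBAL_MESH, and the older line-trace path is unused.
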(event Custom|TriggerLeftSpawnEvent
  (params (Triggered :type Boolean) (Started :type Boolean) (Ongoing :type Boolean) (Canceled :type Boolean) (Completed :type Boolean) (Value :type Boolean) (Action :type Object%20Object%20Reference))
  (bind _newtransform (CallFunction|GetObjectPreviewTransform))
  (Utilities|FlowControl|Sequence
    (:then_0
      (Audio|PlaySound2D "/Game/Static/2_SFX/AirpodsSFX/SC_Airpods.SC_Airpods" 1.0 1.0 0.0 0 0)
      (Rendering|SetVisibility (Variables|Default|GetObjectPreview) Value false)
      (Utilities|RaycastforAnchors
        (:Else
          (Rendering|SetVisibility (Variables|Default|GetObjectPreview) false false))))
    (:then_1
      (if Completed
        (bind _bp_spawnedobj (Variables|Default|GetBP_SpawnedObj)
          (:then
            (Transformation|SetWorldTransform (Variables|/Script/Engine.Actor|GetRootComponent _bp_spawnedobj) _newtransform false true)
            (Audio|Components|Audio|Play (Variables|Default|Getui_open) 0.0)
            (Class|MetaXRHapticsPlayerComponent|PlayonController (Variables|Default|GetMetaXRHapticsPlayer_ui_open) "Left"))
          (:else
            (bind _returnvalue (Game|SpawnActorfromClass (Variables|Default|GetClassToBeSpawned) _newtransform "Undefined" "MultiplyWithRoot" 0 0))
            (Variables|Default|SetBP_SpawnedObj _returnvalue)
            (Audio|Components|Audio|Play (Variables|Default|Getui_open) 0.0)
            (Class|MetaXRHapticsPlayerComponent|PlayonController (Variables|Default|GetMetaXRHapticsPlayer_ui_open) "Left")))))))

(event EventBeginPlay
  ;[0.15 0.15 0.15 0.5] Get ref to AC_GameManager
  (bind _asvrpawn (Utilities|Casting|CastToVRPawn (Game|Player|GetPlayerPawn 0)))
  (bind _output_get (Variables|Default|SetAC%20Game%20Manager (Variables|/Game/Dynamic/1_MixedReality/VRPawn.VRPawn_C|GetAC_GameManager _asvrpawn)))
  (EventDispatchers|BindEventtoLeftTriggerEvent _output_get (delegate Custom|TriggerLeftSpawnEvent))
  (Variables|Default|SetMotion%20Controller%20Right%20Aim (Variables|/Game/Dynamic/1_MixedReality/VRPawn.VRPawn_C|GetMotionControllerLeftAim _asvrpawn)))

(fn ConstructionScript)

(fn RaycastforAnchors
  (params (Start :type Vector) (End :type Vector))
  (bind _outhits (Class|KismetSystemLibrary|LineTraceMultiforObjects Start End (Utilities|Array|MakeArray "ObjectTypeQuery2") false 0 "ForOneFrame" true))
  (for _array_element _outhits
    (Utilities|IsValid (Actor|GetComponentbyClass (.hitactor _array_element) "/Script/OculusXRScene.OculusXRSceneAnchorComponent")
      (:Is%20Valid
        (Development|PrintString " 
 
 
 
 
 
 
 
 
 
 
 
 
trace hit!")
        (return (Actor|GetComponentbyClass (.hitactor _array_element) "/Script/OculusXRScene.OculusXRSceneAnchorComponent") (.impactpoint _array_element) true (.hitcomponent _array_element) (.normal _array_element)))))
  (Development|PrintString " 
 
 
 
 
 
 
 
 
 
 
 
 
trace miss!")
  (return 0 "0, 0, 0" false 0 "0, 0, 0"))

(fn RayforLineTrace
  (params (Start%20In :type Vector) (Direction%20In :type Vector))
  (return Start%20In (+ Start%20In (* Direction%20In 999))))

(fn CalcIndicatorRotation
  (bind _defaultsceneroot (Variables|Default|GetDefaultSceneRoot))
  (bind _returnvalue (Math|Vector|GetForwardVector _defaultsceneroot))
  (bind _returnvalue_2 (Math|Vector|MakeVector (.x _returnvalue) (.y _returnvalue) 0.0))
  (bind _returnvalue_3 (Math|Rotator|MakeRotfromX _returnvalue_2))
  (return (Math|Rotator|MakeRotator (.roll _returnvalue_3) (.pitch _returnvalue_3) (|(x+90) (.yaw _returnvalue_3)))))

(fn RaycastforAnchorswithMRUK
  (bind _motion_controller_right_aim (Variables|Default|GetMotion%20Controller%20Right%20Aim))
  (bind (_outhit _returnvalue) (Class|MRUKSubsystem|Raycast (Subsystems|GetMRUKSubsystem) (Transformation|GetWorldLocation _motion_controller_right_aim) (Math|Vector|GetForwardVector _motion_controller_right_aim) 0.0))
  (Utilities|IsValid _returnvalue
    (:Is%20Valid
      (Development|PrintString " 
 
 
Raycast Hit!")
      (if (Variables|Default|GetOnlySpawnOnTheFloor)
        (if (Utilities|Array|ContainsItem (Variables|/Script/MRUtilityKit.MRUKAnchor|GetSemanticClassifications _returnvalue) "GLOBAL_MESH")
          (Development|PrintString " 
 
 
Found Floor")
          (for _array_element 0
            (Development|PrintString _array_element))
          (return (.HitPosition (Utilities|Struct|BreakMRUKHit _outhit)) (.HitNormal (Utilities|Struct|BreakMRUKHit _outhit)) true)
          (else
            (Development|PrintString " 
 
 
 
Does Not Found Floor")
            (for _array_element_2 (Variables|/Script/MRUtilityKit.MRUKAnchor|GetSemanticClassifications _returnvalue)
              (Development|PrintString _array_element_2))))
        (else
          (return (.HitPosition (Utilities|Struct|BreakMRUKHit _outhit)) (.HitNormal (Utilities|Struct|BreakMRUKHit _outhit)) true))))
    (:Is%20Not%20Valid
      (return "0, 0, 0" "0, 0, 0" false))))

(fn GetRotationBasedonPlayerPOS
  (bind _asvrpawn (Utilities|Casting|CastToVRPawn (Game|Player|GetPlayerPawn 0)))
  (return (Math|Rotator|FindLookatRotation (.location (Transformation|GetWorldTransform (Variables|Default|GetObjectPreview))) (Transformation|GetWorldLocation (Variables|/Game/Dynamic/1_MixedReality/VRPawn.VRPawn_C|GetWidgetInteractionRight _asvrpawn)))))

(fn GetObjectPreviewTransform
  (bind _objectpreview (Variables|Default|GetObjectPreview))
  (bind _returnvalue (Transformation|GetWorldTransform _objectpreview))
  (return (Math|Transform|MakeTransform (.location _returnvalue) (Math|Rotator|MakeRotator 0.0 0.0 (.yaw (Transformation|GetWorldRotation (Variables|Default|GetIndicator)))) (.scale _returnvalue))))