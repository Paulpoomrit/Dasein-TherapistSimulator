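; Mixed-reality game manager component that drives startup from Android permission checks in packaged builds to populating the scanned room.
; It spawns the main menu at the camera with background music, broadcasting dispatchers as stages complete.
; The safety screen timer removes the menu, spawns MRUK anchor actors and places a pistol at the bed anchor, signalling MetaHuman readiness.
; Helper functions switch collision between global mesh and spawned interior actors.
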(event Custom|PermissionGrantedResult
  (params (Permissions :type Array%20of%20Strings) (GrantResults :type Array%20of%20Booleans))
  ;[0.15 0.15 0.15 0.5] Ask for permissions if not exists.
  (if (Utilities|Array|Get(acopy) GrantResults 2)
    (Development|PrintString " 
 
 
 
 
 
 
 
 
 
 
 
 
Has All Permissions.")
    (else
      (Development|PrintString " 
 
 
 
 
 
 
 
 
 
 
Failed To Request Permissions.")
      (Default|CallFailPermissions)))
  ;[0.15 0.15 0.15 0.5] Spawn main menu after 1 sec (this is for BP to property get the camera pos).
  (Utilities|FlowControl|Delay 1.0)
  (CallFunction|SpawnMainMenu))

(event Custom|TimerComplete_Event
  (Actor|DestroyActor (stale Custom|SpawnMainMenu _output_get))
  (Variables|Default|SetSpawnedUMGActor 0)
  (Default|CallSpawnRoomData)
  (CallFunction|SpawnRoomDataEvent))

(event Custom|SpawnMainMenu
  (bind _returnvalue (Game|GetPlayerCameraManager 0))
  (bind _rootcomponent (Variables|/Script/Engine.Actor|GetRootComponent _returnvalue))
  (CallFunction|HandleSound)
  ;[0.15 0.15 0.15 0.5] Spawn Main Menu
  (bind _returnvalue_2 (Game|SpawnActorfromClass "/Game/Dynamic/3_Widgets/1_MainUMG/BP_UMGDisplay.BP_UMGDisplay_C" (Math|Transform|MakeTransform (Transformation|GetWorldLocation _rootcomponent) (Transformation|GetWorldRotation _rootcomponent) "1.000000,1.000000,1.000000") "Undefined" "MultiplyWithRoot" 0 0))
  (bind _output_get (Variables|Default|SetSpawnedUMGActor _returnvalue_2))
  ;[0.15 0.15 0.15 0.5] Tell other actors: main menu is spawned!
  (Default|CallSpawnedMainMenu)
  (bind _aswbp_main_menu_master (Utilities|Casting|CastToWBP_MainMenuMaster (UserInterface|GetWidget (Variables|/Game/Dynamic/3_Widgets/1_MainUMG/BP_UMGDisplay.BP_UMGDisplay_C|GetWidget _output_get))))
  (EventDispatchers|AssignTimerComplete (Variables|/Game/Dynamic/3_Widgets/1_MainUMG/WBP_MainMenuMaster.WBP_MainMenuMaster_C|GetWBP_SafetyScreen _aswbp_main_menu_master) (delegate Custom|TimerComplete_Event)))

(event Custom|SpawnDynamicActors
  (bind _returnvalue (Subsystems|GetMRUKSubsystem))
  (bind _returnvalue_2 (Class|MRUKSubsystem|GetCurrentRoom _returnvalue))
  (bind _returnvalue_3 (Class|MRUKRoom|GetAnchorsbyLabel _returnvalue_2 "BED"))
  (bind _output (Utilities|Array|Get(acopy) _returnvalue_3))
  ;[0.15 0.15 0.15 0.5] Spawn actor using room anchor labels
  (Utilities|IsValid _output
    (:Is%20Valid
      (Game|SpawnActorfromClass "/Game/Static/VRTemplate/Blueprints/Pistol.Pistol_C" (Math|Transform|MakeTransform (Transformation|GetActorLocation _output) "0, 0, 0" "1.000000,1.000000,1.000000") "Undefined" "MultiplyWithRoot" 0 0)
      (Default|CallSceneReadyforSpawningMetahuman))))

(event Custom|SpawnRoomDataEvent
  (bind _returnvalue (Actor|GetActorOfClass "/Script/MRUtilityKit.MRUKAnchorActorSpawner"))
  (Class|MRUKAnchorActorSpawner|SpawnActors _returnvalue (Class|MRUKSubsystem|GetCurrentRoom (Subsystems|GetMRUKSubsystem)))
  (CallFunction|SpawnDynamicActors))

(event EventBeginPlay
  (bind _array (Utilities|Array|MakeArray "android.permission.WRITE_EXTERNAL_STORAGE" "android.permission.READ_EXTERNAL_STORAGE" "com.oculus.permission.USE_SCENE"))
  ;[0.15 0.15 0.15 0.5] if still in development -> skip to main menu!
  (if (Class|KismetSystemLibrary|IsPackagedforDistribution)
    ;[0.15 0.15 0.15 0.5] Check Android Permissions
    (for (_array_element _array_index) _array
      (bind _returnvalue (Class|AndroidPermissionFunctionLibrary|CheckPermission _array_element))
      (if _returnvalue
        ;[0.15 0.15 0.15 0.5] Check all permissions
        (bind _returnvalue_2 (Utilities|Array|Add (Variables|Default|GetNumberOfPermissionsGranted) _array_index))
        (Development|PrintString (Utilities|String|ToString(Integer) _returnvalue_2))
        (if (== _returnvalue_2 2)
          (Development|PrintString " 
 
 
 
 
 
 
 
 
 
 
 
 
Has All Permissions.")
          (else
            (Development|PrintString " 
 
 
 
 
 
 
 
 
 
 
Failed To Request Permissions.")
            (Default|CallFailPermissions)))
        ;[0.15 0.15 0.15 0.5] Spawn main menu after 1 sec (this is for BP to property get the camera pos).
        (Utilities|FlowControl|Delay 1.0)
        (CallFunction|SpawnMainMenu)
        (else
          ;[0.15 0.15 0.15 0.5] Ask for permissions if not exists.
          (bind _returnvalue_3 (Class|AndroidPermissionFunctionLibrary|AcquirePermissions _array))
          (EventDispatchers|BindEventtoOnPermissionsGrantedDynamicDelegate _returnvalue_3 (delegate Custom|PermissionGrantedResult)))))
    (else
      (Utilities|FlowControl|Delay 1.0)
      (CallFunction|SpawnMainMenu))))

(fn HandleSound
  (bind _returnvalue (Audio|SpawnSound2D "/Game/Static/1_Music/Yotam_Agam_-_Unconscious_Mind_Delta.Yotam_Agam_-_Unconscious_Mind_Delta" 1.0 1.0 0.0 0))
  (Variables|Default|SetBackgroundMusic _returnvalue))

(fn EnableGlobalMeshCollision
  (params (Enable :type Boolean))
  (bind _returnvalue (Subsystems|GetMRUKSubsystem))
  (bind _returnvalue_2 (Class|MRUKSubsystem|GetCurrentRoom _returnvalue))
  (CallFunction|EnableInteriorCollision (not Enable))
  (Utilities|IsValid _returnvalue_2
    (:Is%20Valid
      (Utilities|IsValid (Variables|/Script/MRUtilityKit.MRUKRoom|GetGlobalMeshAnchor _returnvalue_2)
        (:Is%20Valid
          (Collision|SetActorEnableCollision (Variables|/Script/MRUtilityKit.MRUKRoom|GetGlobalMeshAnchor (Class|MRUKSubsystem|GetCurrentRoom (Subsystems|GetMRUKSubsystem))) Enable)
          (return))))))

(fn EnableInteriorCollision
  (params (Enable :type Boolean))
  (bind _returnvalue (Actor|GetActorOfClass "/Script/MRUtilityKit.MRUKAnchorActorSpawner"))
  (bind _actors (Class|MRUKAnchorActorSpawner|GetSpawnedActors _returnvalue))
  (for _array_element _actors
    (Collision|SetActorEnableCollision _array_element Enable))
  (bind _output_get (LocalVariables|SetCurrentRoom 0))
  (Utilities|IsValid _output_get
    (:Is%20Valid
      (for _array_element_2 (Variables|/Script/MRUtilityKit.MRUKRoom|GetWallAnchors _output_get)
        (Collision|SetActorEnableCollision _array_element_2 Enable))
      (Collision|SetActorEnableCollision (Variables|/Script/MRUtilityKit.MRUKRoom|GetFloorAnchor (LocalVariables|GetCurrentRoom)) Enable)
      (Collision|SetActorEnableCollision (Variables|/Script/MRUtilityKit.MRUKRoom|GetCeilingAnchor (LocalVariables|GetCurrentRoom)) Enable)
      (return))))