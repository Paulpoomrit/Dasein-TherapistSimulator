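; BP_PermissionsCube is a mixed reality actor whose cube shows the result of a permissions check.
; On BeginPlay it binds to the permission success and failure events on ACGameManager.
; Success turns the cube green, waits briefly, then tells the manager to begin the project session.
; Failure turns it red and does nothing further.
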(event Custom|HasPermissions_Event
  (Rendering|Material|SetMaterial (Variables|Default|GetCube) 0 "/Game/Static/VRTemplate/Materials/MI_PermissionGreen.MI_PermissionGreen")
  (Utilities|FlowControl|Delay 2.0)
  (Default|BeginProjectSession (Variables|Default|GetAC_GameManager)))

(event Custom|FailPermissions_Event
  (Rendering|Material|SetMaterial (Variables|Default|GetCube) 0 "/Game/Static/VRTemplate/Materials/MI_PermissionRed.MI_PermissionRed"))

(event EventBeginPlay
  (bind _ac_gamemanager (Variables|Default|GetAC_GameManager))
  (EventDispatchers|AssignHasPermissions _ac_gamemanager (delegate Custom|HasPermissions_Event))
  (EventDispatchers|BindEventtoFailPermissions _ac_gamemanager (delegate Custom|FailPermissions_Event)))

(event Collision|EventActorBeginOverlap
  (params (OtherActor :type Actor%20Object%20Reference)))

(event EventTick
  (params (DeltaSeconds :type Float%20%28single-precision%29)))

(fn ConstructionScript)