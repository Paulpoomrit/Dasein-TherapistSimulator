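; Widget component that shows a Convai chatbot conversation as chat bubbles on a 3D chat widget.
; One tick after BeginPlay it caches its WBP_3DChatWidget and binds to the owner's ConvaiChatbotComponent text, transcription and failure events.
; Bot replies and named player transcriptions update color-coded bubbles with final-state flags.
; Failures post an error bubble whose wording depends on whether the build is packaged for distribution.
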(event EventBeginPlay
  (Utilities|FlowControl|DelayUntilNextTick)
  (bind _aswbp_3dchat_widget (Utilities|Casting|CastToWBP_3DChatWidget (UserInterface|GetWidget)))
  (Variables|Default|Set3DChatWidget _aswbp_3dchat_widget)
  (bind _output_get (Variables|Default|SetOwnerChatbotComp (Actor|GetComponentbyClass (Components|GetOwner) "/Script/Convai.ConvaiChatbotComponent")))
  (|Setupwidgetbindings _output_get))

(event EventTick
  (params (DeltaSeconds :type Float%20%28single-precision%29)))

(event Custom|OnTextReceived
  (params (ChatbotComponent :type Convai%20Chatbot%20Component%20Object%20Reference) (InteractingPlayerComponent :type Convai%20Player%20Component%20Object%20Reference) (CharacterName :type String) (BotText :type String) (AudioDuration :type Float%20%28single-precision%29) (IsFinal :type Boolean))
  (bind _3dchatwidget (Variables|Default|Get3DChatWidget))
  ;[0.1834 1 0] Bind the events needed to show the chat bubbles
  (Utilities|IsValid _3dchatwidget
    (:Is%20Valid
      (Default|AddorUpdateNewChatBubble _3dchatwidget CharacterName BotText (Utilities|Struct|MakeSlateColor "(R=0.000000,G=1.000000,B=0.254000,A=1.000000)") false false IsFinal false false))))

(event Custom|ShowInChatError
  ;[1 0 0] In case a failure happened
  (Utilities|IsValid (Variables|Default|Get3DChatWidget)
    (:Is%20Valid
      (Default|AddorUpdateNewChatBubble (Variables|Default|Get3DChatWidget) "-" (Utilities|String|SelectString "Error! Contact support or check logs." "Error! See logs in Window->Output Log." (Class|KismetSystemLibrary|IsPackagedforDistribution)) (Utilities|Struct|MakeSlateColor "(R=1.000000,G=1.000000,B=0.000000,A=1.000000)") false false true false false))))

(event Custom|OnTranscriptionReceived
  (params (ChatbotComponent :type Convai%20Chatbot%20Component%20Object%20Reference) (InteractingPlayerComponent :type Convai%20Player%20Component%20Object%20Reference) (PlayerName :type String) (Transcription :type String) (IsTranscriptionReady :type Boolean) (IsFinal :type Boolean))
  ;[0.1834 1 0] Bind the events needed to show the chat bubbles
  (Utilities|IsValid InteractingPlayerComponent
    (:Is%20Valid
      (if (not (Utilities|Array|IsEmpty PlayerName))
        (Utilities|IsValid (Variables|Default|Get3DChatWidget)
          (:Is%20Valid
            (Default|AddorUpdateNewChatBubble (Variables|Default|Get3DChatWidget) PlayerName Transcription (Utilities|Struct|MakeSlateColor "(R=1.000000,G=0.250000,B=1.000000,A=1.000000)") true IsTranscriptionReady IsFinal true false)))))))