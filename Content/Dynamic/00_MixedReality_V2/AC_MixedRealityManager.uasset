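; Mixed reality manager component that switches collision between the MRUK global mesh and the interior scene anchors.
; EnableGlobalMeshCollision sets collision on the current room's global mesh anchor and applies the opposite state through EnableInteriorCollision.
; EnableInteriorCollision toggles every actor from the MRUK anchor actor spawner.
; Its wall, floor and ceiling branch reads an unset room reference, so it never runs.
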(event EventBeginPlay)

(event EventTick
  (params (DeltaSeconds :type Float%20%28single-precision%29)))

(fn EnableGlobalMeshCollision
  (params (Enable :type Boolean))
  (bind _returnvalue (Subsystems|GetMRUKSubsystem))
  (bind _returnvalue_2 (Class|MRUKSubsystem|GetCurrentRoom _returnvalue))
  (CallFunction|EnableInteriorCollision (not Enable))
  (Utilities|IsValid _returnvalue_2
    (:Is%20Valid
      (Utilities|IsValid (Variables|/Script/MRUtilityKit.MRUKRoom|GetGlobalMeshAnchor _returnvalue_2)
        (:Is%20Valid
          (Collision|SetActorEnableCollision (Variables|/Script/MRUtilityKit.MRUKRoom|GetGlobalMeshAnchor (Class|MRUKSubsystem|GetCurrentRoom (Subsystems|GetMRUKSubsystem))) Enable)
          (return))))))

(fn EnableInteriorCollision
  (params (Enable :type Boolean))
  (bind _returnvalue (Actor|GetActorOfClass "/Script/MRUtilityKit.MRUKAnchorActorSpawner"))
  (bind _actors (Class|MRUKAnchorActorSpawner|GetSpawnedActors _returnvalue))
  (for _array_element _actors
    (Collision|SetActorEnableCollision _array_element Enable))
  (bind _output_get (LocalVariables|SetCurrentRoom 0))
  (Utilities|IsValid _output_get
    (:Is%20Valid
      (for _array_element_2 (Variables|/Script/MRUtilityKit.MRUKRoom|GetWallAnchors _output_get)
        (Collision|SetActorEnableCollision _array_element_2 Enable))
      (Collision|SetActorEnableCollision (Variables|/Script/MRUtilityKit.MRUKRoom|GetFloorAnchor (LocalVariables|GetCurrentRoom)) Enable)
      (Collision|SetActorEnableCollision (Variables|/Script/MRUtilityKit.MRUKRoom|GetCeilingAnchor (LocalVariables|GetCurrentRoom)) Enable)
      (return))))