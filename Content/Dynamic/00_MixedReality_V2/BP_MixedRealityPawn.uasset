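; Mixed reality VR pawn that shows Meta (OculusXR) passthrough and relays left-trigger input to the game manager.
; On BeginPlay, if an HMD is enabled, it sets view-relative tracking, adds VR, hand and mixed reality input contexts, and initializes persistent passthrough.
; The collapsed StartSpawning_2 graph forwards each IA_TriggerLeft phase to AC_GameManager, intended to start spawning.
; Older direct trigger calls and start/stop talking nodes remain disconnected.
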(event Input|EnhancedActionEvents|EnhancedInputActionIA_TriggerLeft
  (params (ActionValue :type Boolean) (ElapsedSeconds :type Float%20%28double-precision%29) (TriggeredSeconds :type Float%20%28double-precision%29) (InputAction :type Input%20Action%20Object%20Reference :default "/Game/Dynamic/1_MixedReality/Input/Actions/IA_TriggerLeft.IA_TriggerLeft"))
  ;[0 0.1019 0.15 0.5] Trigger Left to Start Spawning Things (send info to AC_GameManager)
  (:Triggered
    (|StartSpawning_2 ActionValue ActionValue ActionValue ActionValue ActionValue InputAction InputAction InputAction InputAction InputAction :!label _label))
  (:Started
    (goto _label execute4))
  (:Ongoing
    (goto _label execute2))
  (:Canceled
    (goto _label execute5))
  (:Completed
    (goto _label execute3)))

(event Input|EnhancedActionEvents|EnhancedInputActionIA_TriggerLeft_V2
  (params (ActionValue :type Boolean) (ElapsedSeconds :type Float%20%28double-precision%29) (TriggeredSeconds :type Float%20%28double-precision%29) (InputAction :type Input%20Action%20Object%20Reference :default "/Game/Dynamic/00_MixedReality_V2/Inputs/IA_TriggerLeft_V2.IA_TriggerLeft_V2")))

(event EventBeginPlay
  (bind _returnvalue (Game|GetPlayerController 0))
  (bind _returnvalue_2 (PlayerController|LocalPlayerSubsystems|GetEnhancedInputLocalPlayerSubsystem _returnvalue))
  (if (Class|HeadMountedDisplayFunctionLibrary|IsHeadMountedDisplayEnabled)
    (Class|HeadMountedDisplayFunctionLibrary|SetTrackingOrigin "View")
    (Input|AddMappingContext _returnvalue_2 "/Game/Dynamic/1_MixedReality/Input/IMC_VR_Default.IMC_VR_Default" 5 "(bIgnoreAllPressedKeysUntilRelease=True,bForceImmediately=False,bNotifyUserSettings=False)")
    (Input|AddMappingContext _returnvalue_2 "/Game/Dynamic/1_MixedReality/Input/IMC_Hands.IMC_Hands" 1 "(bIgnoreAllPressedKeysUntilRelease=True,bForceImmediately=False,bNotifyUserSettings=False)")
    (Input|AddMappingContext _returnvalue_2 "/Game/Dynamic/00_MixedReality_V2/Inputs/IMC_MixedRealityDefault.IMC_MixedRealityDefault" 2 "(bIgnoreAllPressedKeysUntilRelease=True,bForceImmediately=False,bNotifyUserSettings=False)")
    ;[0.15 0.15 0.15 0.5] enable passthrough
    (bind _returnvalue_3 (Class|OculusXRPassthroughSubsystem|InitializePersistentPassthrough (Subsystems|GetOculusXRPassthroughSubsystem)))
    (Variables|Default|SetPersistentPassthrough _returnvalue_3)))

(fn ConstructionScript)