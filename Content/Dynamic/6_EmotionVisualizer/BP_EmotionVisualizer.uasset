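; Emotion visualizer actor that shows a chatbot's dominant emotion through a coloured, spinning orb and a text widget.
; On BeginPlay it creates a dynamic material for the orb and caches the text widget, while Tick rotates the root.
; SetVisualizerMaterialColour picks the highest-scoring emotion from the passed-in chatbot, with ties going to the later enum entry.
; It then recolours the orb, writes the emotion name in black, and prints debug output.
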(event EventBeginPlay
  (bind _returnvalue (Rendering|Material|CreateDynamicMaterialInstance (Variables|Default|GetOrb) 1 "/Game/Static/Clinic/Materials/MaterialInstances/MI_Lights.MI_Lights" "None" :!class /Script/Engine.PrimitiveComponent))
  (Variables|Default|SetMaterialColour _returnvalue)
  (bind _aswbp_emotion_text (Utilities|Casting|CastToWBP_EmotionText (UserInterface|GetWidget (Variables|Default|GetEmotionText))))
  (Variables|Default|SetEmotion%20Text _aswbp_emotion_text))

(event EventTick
  (params (DeltaSeconds :type Float%20%28single-precision%29))
  (Transformation|AddLocalRotation (Variables|Default|Getroot) (Math|Rotator|MakeRotator 0.0 0.0 (* DeltaSeconds (Variables|Default|GetRotation))) false false))

(fn ConstructionScript)

(fn FindDominantEmotion
  (params (Chatbot :type Convai%20Chatbot%20Component%20Object%20Reference))
  (LocalVariables|SetMaxEmotionScore 0.0)
  (LocalVariables|SetDominantEmotion (Variables|Default|GetCurrentEmotion))
  (bind _enumvalue (|ForEachEBasicEmotions)
    (:LoopBody
      (if (>= (Class|ConvaiChatbotComponent|GetEmotionScore Chatbot _enumvalue) (LocalVariables|GetMaxEmotionScore))
        (LocalVariables|SetMaxEmotionScore (Class|ConvaiChatbotComponent|GetEmotionScore Chatbot _enumvalue))
        (LocalVariables|SetDominantEmotion _enumvalue)))
    (:then
      (return (LocalVariables|GetDominantEmotion) (LocalVariables|GetMaxEmotionScore)))))

(fn SetVisualizerMaterialColour
  (params (Chatbot :type Convai%20Chatbot%20Component%20Object%20Reference))
  (bind (_emotion _score) (CallFunction|FindDominantEmotion Chatbot))
  (Variables|Default|SetCurrentEmotion _emotion)
  (Development|PrintString (Utilities|String|EnumtoString _emotion))
  (Development|PrintString (Utilities|String|ToString(Float) _score))
  (switch Utilities|FlowControl|Switch|SwitchonEBasicEmotions _emotion
    (:Joy
      (Rendering|Material|SetVectorParameterValue (Variables|Default|GetMaterialColour) "Color" "(R=0.041786,G=1.000000,B=0.000000,A=1.000000)" :!class /Script/Engine.MaterialInstanceDynamic))
    (:Trust
      (Rendering|Material|SetVectorParameterValue (Variables|Default|GetMaterialColour) "Color" "(R=0.000000,G=1.000000,B=0.898629,A=1.000000)" :!class /Script/Engine.MaterialInstanceDynamic))
    (:Fear
      (Rendering|Material|SetVectorParameterValue (Variables|Default|GetMaterialColour) "Color" "(R=0.386517,G=0.000000,B=1.000000,A=1.000000)" :!class /Script/Engine.MaterialInstanceDynamic))
    (:Surprise
      (Rendering|Material|SetVectorParameterValue (Variables|Default|GetMaterialColour) "Color" "(R=1.000000,G=0.700182,B=0.025944,A=1.000000)" :!class /Script/Engine.MaterialInstanceDynamic))
    (:Sadness
      (Rendering|Material|SetVectorParameterValue (Variables|Default|GetMaterialColour) "Color" "(R=0.838197,G=0.000000,B=1.000000,A=1.000000)" :!class /Script/Engine.MaterialInstanceDynamic))
    (:Disgust
      (Rendering|Material|SetVectorParameterValue (Variables|Default|GetMaterialColour) "Color" "(R=0.000000,G=0.000000,B=0.000000,A=1.000000)" :!class /Script/Engine.MaterialInstanceDynamic))
    (:Anger
      (Rendering|Material|SetVectorParameterValue (Variables|Default|GetMaterialColour) "Color" "(R=1.000000,G=0.000000,B=0.099285,A=1.000000)" :!class /Script/Engine.MaterialInstanceDynamic)))
  (Rendering|Material|GetVectorParameterValue (Variables|Default|GetMaterialColour) "Color" :!class /Script/Engine.MaterialInstanceDynamic)
  (Default|SetTextContentandColor (Variables|Default|GetEmotion%20Text) (Utilities|Text|ToText(String) (Utilities|String|EnumtoString _emotion)) (Utilities|Struct|MakeSlateColor "(R=0.000000,G=0.000000,B=0.000000,A=1.000000)" "UseColor_Specified")))